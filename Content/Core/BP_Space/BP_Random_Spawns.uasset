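; BP_Random_Spawns is a spawner actor that scatters random pawns from its Planets class array throughout a box volume.
; On BeginPlay a fixed loop picks a random class each pass and calls SpawnAIFromClass at a random point within the Box extent, centred on DefaultSceneRoot.
; Spawns ignore collision failure, and each pass also prints a leftover-looking "Hello" debug string.
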(event EventBeginPlay
  (bind _planets (Variables|Default|GetPlanets))
  (for _index (range 0 10)
    (Development|PrintString "Hello")
    (AI|SpawnAIFromClass (Utilities|Array|Get(acopy) _planets (Math|Random|RandomIntegerinRange 0 (- (Utilities|Array|Length _planets) 1))) 0 (Math|Random|RandomPointinBoundingBox (Transformation|GetWorldLocation (Variables|Default|GetDefaultSceneRoot)) (Variables|/Script/Engine.BoxComponent|GetBoxExtent (Variables|Default|GetBox))) "0, 0, 0" true)))

(event Collision|EventActorBeginOverlap
  (params (OtherActor :type Actor%20Object%20Reference)))

(event EventTick
  (params (DeltaSeconds :type Float%20%28single-precision%29)))

(fn ConstructionScript)