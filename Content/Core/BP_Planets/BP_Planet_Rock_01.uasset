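; BP_Planet_Rock_01 is the rock planet, with a hit handler for collisions with other planets while the player's cue ball is moving.
; On a component hit it checks the cue ball pawn's moving flag, then switches on the other actor's class display name for ice, fire or rock.
; Each branch only casts, with comments deferring ice and fire collisions to those Blueprints.
; The hit component keeps an Ice name, DM_Planet_Ice_01.
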(event OnComponentHit(DM_Planet_Ice_01)
  (params (HitComponent :type Primitive%20Component%20Object%20Reference) (OtherActor :type Actor%20Object%20Reference) (OtherComp :type Primitive%20Component%20Object%20Reference) (NormalImpulse :type Vector :default "0, 0, 0") (Hit :type Hit%20Result%20Structure%20%28by%20ref%29))
  (bind _asbp_cue_ball_01 (Utilities|Casting|CastToBP_Cue_Ball_01 (Game|Player|GetPlayerPawn 0)))
  (if (Variables|/Game/Core/BP_Controller/BP_Cue_Ball_01.BP_Cue_Ball_01_C|GetCue%20Ball%20Moving%20 _asbp_cue_ball_01)
    (switch string (Utilities|GetClassDisplayName (Utilities|GetClass OtherActor))
      (:BP_Planet_Ice_01_C
        ;[1 1 1] Ice Hitting Rock (See BP_Planet_Ice_01)
        (Utilities|Casting|CastToBP_Planet_Ice_01 OtherActor))
      (:BP_Planet_Fire_01_C
        ;[1 1 1] Fire Hitting Rock (See BP_Planet_Fire_01)
        (Utilities|Casting|CastToBP_Planet_Fire_01 OtherActor))
      (:BP_Planet_Rock_01_C
        ;[1 1 1] Rock Hitting Ice
        (Utilities|Casting|CastToBP_Planet_Rock_01 OtherActor)))))

(fn ConstructionScript)