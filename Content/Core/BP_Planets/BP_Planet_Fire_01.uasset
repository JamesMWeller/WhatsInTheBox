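; Fire planet in a cue-ball game that reacts to hits from other planets and awards player points, only while the cue ball is moving.
; On hit it switches on the other actor's class display name: unbroken ice melts via a scale timeline and is destroyed after a delay.
; Rock is replaced by a newly spawned fire planet, while broken ice and other fire planets only add points to the player controller.
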(event OnComponentHit(DM_Planet_Fire_01)
  (params (HitComponent :type Primitive%20Component%20Object%20Reference) (OtherActor :type Actor%20Object%20Reference) (OtherComp :type Primitive%20Component%20Object%20Reference) (NormalImpulse :type Vector :default "0, 0, 0") (Hit :type Hit%20Result%20Structure%20%28by%20ref%29))
  (bind _asbp_cue_ball_01 (Utilities|Casting|CastToBP_Cue_Ball_01 (Game|Player|GetPlayerPawn 0)))
  (if (Variables|/Game/Core/BP_Controller/BP_Cue_Ball_01.BP_Cue_Ball_01_C|GetCue%20Ball%20Moving%20 _asbp_cue_ball_01)
    (switch string (Utilities|GetClassDisplayName (Utilities|GetClass OtherActor))
      (:BP_Planet_Ice_01_C
        ;[1 1 1] Ice Hitting Fire
        (bind _asbp_planet_ice_01 (Utilities|Casting|CastToBP_Planet_Ice_01 OtherActor))
        (if (Variables|/Game/Core/BP_Planets/BP_Planet_Ice_01.BP_Planet_Ice_01_C|GetBroken _asbp_planet_ice_01)
          ;[1 1 1] Broken Ice Hitting Fire
          (bind _asbp_player_controller (Utilities|Casting|CastToBP_Player_Controller (Game|GetPlayerController 0)))
          (Variables|/Game/Core/BP_Controller/BP_Player_Controller.BP_Player_Controller_C|SetPlayer%20Points _asbp_player_controller (+ (Variables|/Game/Core/BP_Controller/BP_Player_Controller.BP_Player_Controller_C|GetPlayer%20Points _asbp_player_controller) 1))
          (elif (not (Variables|/Game/Core/BP_Planets/BP_Planet_Ice_01.BP_Planet_Ice_01_C|GetMelting _asbp_planet_ice_01))
            (Variables|/Game/Core/BP_Planets/BP_Planet_Ice_01.BP_Planet_Ice_01_C|SetMelting _asbp_planet_ice_01 true)
            (bind _size (Timeline|Timeline_0 PlayFromStart)
              (:Update
                (Transformation|SetRelativeScale3D (Variables|/Game/Core/BP_Planets/BP_Planet_Ice_01.BP_Planet_Ice_01_C|GetDM_Planet_Ice_01 _asbp_planet_ice_01) _size))
              (:Finished
                (Utilities|FlowControl|Delay 1.0)
                (Actor|DestroyActor _asbp_planet_ice_01)
                (bind _asbp_player_controller_2 (Utilities|Casting|CastToBP_Player_Controller (Game|GetPlayerController 0)))
                (Variables|/Game/Core/BP_Controller/BP_Player_Controller.BP_Player_Controller_C|SetPlayer%20Points _asbp_player_controller_2 (+ (Variables|/Game/Core/BP_Controller/BP_Player_Controller.BP_Player_Controller_C|GetPlayer%20Points _asbp_player_controller_2) 10)))))))
      (:BP_Planet_Fire_01_C
        ;[1 1 1] Fire Hitting Fire
        (Utilities|Casting|CastToBP_Planet_Fire_01 OtherActor)
        (bind _asbp_player_controller_3 (Utilities|Casting|CastToBP_Player_Controller (Game|GetPlayerController 0)))
        (Variables|/Game/Core/BP_Controller/BP_Player_Controller.BP_Player_Controller_C|SetPlayer%20Points _asbp_player_controller_3 (+ (Variables|/Game/Core/BP_Controller/BP_Player_Controller.BP_Player_Controller_C|GetPlayer%20Points _asbp_player_controller_3) 1)))
      (:BP_Planet_Rock_01_C
        ;[1 1 1] Rock Hitting Fire
        (bind _asbp_planet_rock_01 (Utilities|Casting|CastToBP_Planet_Rock_01 OtherActor))
        (AI|SpawnAIFromClass "BP_Planet_Fire_01_C" 0 (Transformation|GetWorldLocation (Variables|/Game/Core/BP_Planets/BP_Planet_Rock_01.BP_Planet_Rock_01_C|GetDM_Planet_Rock_01 _asbp_planet_rock_01)) "0, 0, 0" true)
        (Actor|DestroyActor _asbp_planet_rock_01)
        (bind _asbp_player_controller_4 (Utilities|Casting|CastToBP_Player_Controller (Game|GetPlayerController 0)))
        (Variables|/Game/Core/BP_Controller/BP_Player_Controller.BP_Player_Controller_C|SetPlayer%20Points _asbp_player_controller_4 (+ (Variables|/Game/Core/BP_Controller/BP_Player_Controller.BP_Player_Controller_C|GetPlayer%20Points _asbp_player_controller_4) 2))))))

(fn ConstructionScript)