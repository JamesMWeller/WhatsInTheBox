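; BP_Planet_Ice_01 is an ice planet with a destructible mesh that reacts to collisions and awards points while the cue ball is moving.
; On hit, it branches on the other actor's class name, adding a small score for ice contact and leaving fire contact to BP_Planet_Fire_01.
; A rock hit fractures the mesh, sets Broken, adds a larger score to BP_Player_Controller and destroys the actor after a delay.
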(event OnComponentHit(DM_Planet_Ice_01)
  (params (HitComponent :type Primitive%20Component%20Object%20Reference) (OtherActor :type Actor%20Object%20Reference) (OtherComp :type Primitive%20Component%20Object%20Reference) (NormalImpulse :type Vector :default "0, 0, 0") (Hit :type Hit%20Result%20Structure%20%28by%20ref%29))
  (bind (_bblockinghit _binitialoverlap _time _distance _location _impactpoint _normal _impactnormal) (Collision|BreakHitResult Hit))
  (bind _asbp_cue_ball_01 (Utilities|Casting|CastToBP_Cue_Ball_01 (Game|Player|GetPlayerPawn 0)))
  (if (Variables|/Game/Core/BP_Controller/BP_Cue_Ball_01.BP_Cue_Ball_01_C|GetCue%20Ball%20Moving%20 _asbp_cue_ball_01)
    (switch string (Utilities|GetClassDisplayName (Utilities|GetClass OtherActor))
      (:BP_Planet_Ice_01_C
        ;[1 1 1] Ice Hitting Ice
        (Utilities|Casting|CastToBP_Planet_Ice_01 OtherActor)
        (bind _asbp_player_controller (Utilities|Casting|CastToBP_Player_Controller (Game|GetPlayerController 0)))
        (Variables|/Game/Core/BP_Controller/BP_Player_Controller.BP_Player_Controller_C|SetPlayer%20Points _asbp_player_controller (+ (Variables|/Game/Core/BP_Controller/BP_Player_Controller.BP_Player_Controller_C|GetPlayer%20Points _asbp_player_controller) 2)))
      (:BP_Planet_Fire_01_C
        ;[1 1 1] Fire Hitting Ice (See BP_Planet_Fire_01)
        (Utilities|Casting|CastToBP_Planet_Fire_01 OtherActor))
      (:BP_Planet_Rock_01_C
        ;[1 1 1] Rock Hitting Ice
        (Utilities|Casting|CastToBP_Planet_Rock_01 OtherActor)
        (Class|DestructibleComponent|ApplyDamage (Variables|Default|GetDM_Planet_Ice_01) 1.0 _impactpoint _impactnormal 0.0)
        (Variables|Default|SetBroken true)
        (bind _asbp_player_controller_2 (Utilities|Casting|CastToBP_Player_Controller (Game|GetPlayerController 0)))
        (Variables|/Game/Core/BP_Controller/BP_Player_Controller.BP_Player_Controller_C|SetPlayer%20Points _asbp_player_controller_2 (+ (Variables|/Game/Core/BP_Controller/BP_Player_Controller.BP_Player_Controller_C|GetPlayer%20Points _asbp_player_controller_2) 10))
        (Utilities|FlowControl|Delay 4.0)
        (Actor|DestroyActor)))))

(fn ConstructionScript)