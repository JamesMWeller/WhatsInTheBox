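; Intro camera actor that flies a camera along a spline, then loads the CoreGame level.
; On BeginPlay, the Camera_Move timeline maps its AnimAlpha to distance along the spline, setting the camera's world location and rotation each update.
; A camera fade starts only when alpha exactly equals 0.7, a float comparison that may never match.
; Timeline completion opens the level.
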(event Collision|EventActorBeginOverlap
  (params (OtherActor :type Actor%20Object%20Reference)))

(event EventTick
  (params (DeltaSeconds :type Float%20%28single-precision%29)))

(event EventBeginPlay
  (bind _spline (Variables|Default|GetSpline))
  (bind _anim_alpha (Timeline|Camera_Move PlayFromStart)
    (:Update
      (Transformation|SetWorldTransform (Variables|Default|GetCamera) (Math|Transform|MakeTransform (Spline|GetLocationatDistanceAlongSpline _spline (* (Spline|GetSplineLength _spline) _anim_alpha) "World") (Spline|GetRotationatDistanceAlongSpline _spline (* (Spline|GetSplineLength _spline) _anim_alpha) "World")) false false)
      (if (== _anim_alpha 0.7)
        (CameraFades|StartCameraFade :self (Game|GetPlayerCameraManager 0) :ToAlpha 1.0)))
    (:Finished
      (Game|OpenLevel(byName) "CoreGame"))))

(fn ConstructionScript)