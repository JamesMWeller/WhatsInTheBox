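; Player controller that shoots the cue ball with a left-click charge-and-release.
; Pressing casts the pawn to BP_Cue_Ball_01 and starts a timeline driving Power, while Tick draws a debug aim line.
; Releasing applies an impulse away from the cursor, scaled by Power and cursor-to-ball distance.
; The cursor point comes from intersecting the deprojected mouse ray with the X=0 plane, without a trace.
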(event EventTick
  (params (DeltaSeconds :type Float%20%28single-precision%29))
  (bind _returnvalue (Game|GetPlayerController 0))
  (bind (_worldlocation _worlddirection) (Game|Player|ConvertMouseLocationToWorldSpace _returnvalue))
  ;[1 1 1] Left Mouse move / with power
  (Utilities|FlowControl|Sequence
    (:then_0
      (if (Variables|Default|GetmouseDown)
        (Rendering|Debug|DrawDebugLine (Transformation|GetWorldLocation (Variables|/Game/Core/BP_Controller/BP_Cue_Ball_01.BP_Cue_Ball_01_C|GetBall (stale Input|ActionEvents|InputActionMouseLeftClick _asbp_cue_ball_01))) (+ (Transformation|GetWorldLocation (Variables|/Game/Core/BP_Controller/BP_Cue_Ball_01.BP_Cue_Ball_01_C|GetBall (stale Input|ActionEvents|InputActionMouseLeftClick _asbp_cue_ball_01))) (- (Transformation|GetWorldLocation (Variables|/Game/Core/BP_Controller/BP_Cue_Ball_01.BP_Cue_Ball_01_C|GetBall (stale Input|ActionEvents|InputActionMouseLeftClick _asbp_cue_ball_01))) (+ _worldlocation (* (* _worlddirection (/ (.X (Math|Vector|BreakVector _worldlocation)) (.X (Math|Vector|BreakVector _worlddirection)))) -1.0)))) "(R=0.000000,G=0.190107,B=1.000000,A=1.000000)" 0.0 5.0)))))

(event Input|ActionEvents|InputActionMouseLeftClick
  (params (Key :type Key%20Structure))
  (bind _returnvalue (Game|GetPlayerController 0))
  (bind (_worldlocation _worlddirection) (Game|Player|ConvertMouseLocationToWorldSpace _returnvalue))
  ;[1 1 1] Left Mouse move / with power
  (:Pressed
    (Utilities|FlowControl|Sequence
      (:then_0
        (bind _asbp_cue_ball_01 (Utilities|Casting|CastToBP_Cue_Ball_01 (Game|Player|GetPlayerPawn 0))))
      (:then_1
        (bind _newtrack_0 (Timeline|Timeline_0 PlayFromStart)
          (:Update
            (Variables|Default|SetPower _newtrack_0))))
      (:then_2
        (Variables|Default|SetmouseDown true))))
  (:Released
    (Variables|Default|SetmouseDown false)
    (Physics|AddImpulse (Variables|/Game/Core/BP_Controller/BP_Cue_Ball_01.BP_Cue_Ball_01_C|GetBall _asbp_cue_ball_01) (* (- (Transformation|GetWorldLocation (Variables|/Game/Core/BP_Controller/BP_Cue_Ball_01.BP_Cue_Ball_01_C|GetBall _asbp_cue_ball_01)) (+ _worldlocation (* (* _worlddirection (/ (.X (Math|Vector|BreakVector _worldlocation)) (.X (Math|Vector|BreakVector _worlddirection)))) -1.0))) (* (Variables|Default|GetPower) 1e+02)) "None" false)))

(fn ConstructionScript)